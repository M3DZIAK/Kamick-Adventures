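; Paper2D side-scroller player character with movement, multi-jump, shooting, health and a timed mushroom buff to size and jump power.
; Tick picks a priority-based flipbook, flips the sprite by velocity and pins the actor to Y=0.
; Keyboard and mobile events share jump and attack logic; jumps offset vertical velocity, with squash-and-stretch timelines and effects.
; Damage triggers a color-timeline invulnerability window, while death opens the Menu level.
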(event Custom|BrownMushroomPickUp
  ;[1 1 1] BrownMushroomPickUp
  (bind _changescale (Timeline|PickUpTimeLine PlayFromStart)
    (:Update
      (Transformation|SetActorScale3D (Math|Vector|Lerp(Vector) (Variables|Default|GetactorStartScale) "2.000000,2.000000,2.000000" _changescale)))
    (:Finished
      (Transformation|SetActorScale3D "1.300000,1.300000,1.300000")
      (Variables|Default|SetjumpBuffMultipler (+ (Variables|Default|GetjumpBuffMultipler) 0.3))
      (Variables|Default|SetactorCurrentScale "1.250000,1.250000,1.250000")
      (Utilities|FlowControl|Delay 5.0)
      (bind _changescale_2 (Timeline|Timeline_0 Play)
        (:Update
          (Transformation|SetActorScale3D (Math|Vector|Lerp(Vector) (Variables|Default|GetactorStartScale) "2.000000,2.000000,2.000000" _changescale_2)))
        (:Finished
          (Variables|Default|SetjumpBuffMultipler (- (Variables|Default|GetjumpBuffMultipler) 0.3))
          (bind _output_get (Variables|Default|SetactorCurrentScale (Variables|Default|GetactorStartScale)))
          (Transformation|SetActorScale3D _output_get))))))

(event Custom|moveCharacter%20mobile
  (params (speed :type Float%20%28single-precision%29))
  ;[1 1 1] Movement
  (Pawn|Input|AddMovementInput "1.000000, 0, 0" speed false))

(event Custom|CheckSite
  ;[1 1 1] Check site
  (Math|Float|CompareFloat (.X (Math|Vector|BreakVector (Transformation|GetVelocity))) 0.0
    (:>
      (Transformation|SetRelativeRotation (Variables|Default|GetSprite) "0, 0, 0" false false))
    (:<
      (Transformation|SetRelativeRotation (Variables|Default|GetSprite) "0.000000,180.000000,0.000000" false false))))

(event Custom|Die
  ;[1 1 1] Death
  (Pawn|Components|CharacterMovement|DisableMovement (Variables|Character|GetCharacterMovement))
  (Variables|Default|SetcanShoot false)
  (Variables|Default|SetisDying true)
  (Utilities|FlowControl|Delay 0.4)
  (Variables|Default|SetisDying false)
  (Rendering|SetVisibility (Variables|Default|GetSprite) false true)
  (Utilities|FlowControl|Delay 0.5)
  (Game|OpenLevel(byName) "Menu"))

(event Custom|LandFX
  (bind _bottompoint (Variables|Default|GetBottomPoint))
  (bind _returnvalue (Transformation|GetWorldLocation _bottompoint))
  ;[1 1 1] LandFX
  (Game|SpawnActorfromClass "/Game/BluePrints/Effects/DirtEffect.DirtEffect_C" (Math|Transform|MakeTransform (Math|Vector|MakeVector (.x _returnvalue) (.y _returnvalue) (+ (.z _returnvalue) 13.0)) "0, 0, 0" "1.250000,1.250000,1.250000") "AlwaysSpawn" 0 0)
  (bind _squeeze (Timeline|LandTimeline PlayFromStart)
    (:Update
      (Transformation|SetActorScale3D (Math|Vector|Lerp(Vector) (Variables|Default|GetactorCurrentScale) "1.500000,0.000000,0.750000" _squeeze)))))

(event Custom|JumpMobile
  (bind _returnvalue (Transformation|GetVelocity))
  ;[1 1 1] Jumping
  (if (< (Variables|Default|GetjumpsCount) (Variables|Default|GetmaxJumps))
    (bind _result (Math|Integer|IncrementInt (Variables|Default|GetjumpsCount))
      (:%20%20
        (Variables|Default|SetjumpsCount _result)
        (if (> (.z _returnvalue) 0.0)
          (Character|LaunchCharacter (Math|Vector|MakeVector 0.0 0.0 (+ (* (.z (Transformation|GetVelocity)) -1.0) (* (Variables|Default|GetjumpBuffMultipler) 2.5e+02))) false false)
          (else
            (Character|LaunchCharacter (Math|Vector|MakeVector 0.0 0.0 (+ (Math|Float|Absolute(Float) (.z _returnvalue)) (* (Variables|Default|GetjumpBuffMultipler) 2.5e+02))) false false)))
        (CallFunction|JumpFX)))))

(event Custom|AttackMobile
  (bind _shootpoint (Variables|Default|GetShootPoint))
  ;[1 1 1] Attacking
  (if (Variables|Default|GetcanShoot)
    (Variables|Default|SetcanShoot false)
    (Variables|Default|SetisAttacking true)
    (Game|SpawnActorfromClass "/Game/BluePrints/Attacks/PlayerShoot1.PlayerShoot1_C" (Math|Transform|MakeTransform (Transformation|GetWorldLocation _shootpoint) (Transformation|GetWorldRotation _shootpoint) "0.500000,0.500000,0.500000") "AlwaysSpawn" 0 0)
    (Utilities|FlowControl|Delay 0.2)
    (Variables|Default|SetisAttacking false)
    (Utilities|FlowControl|Delay (- (Variables|Default|GetshootRate) 0.2))
    (Variables|Default|SetcanShoot true)))

(event Custom|JumpFX
  ;[1 1 1] JumpFX
  (if (AI|Components|NavMovement|IsFalling (Variables|Character|GetCharacterMovement))
    (Game|SpawnActorfromClass "/Game/BluePrints/Effects/CloudEffect.CloudEffect_C" (Math|Transform|MakeTransform (Transformation|GetWorldLocation (Variables|Default|GetBottomPoint)) "0, 0, 0" "0.800000,1.000000,0.800000") "AlwaysSpawn" 0 0)
    (bind _squeeze (Timeline|JumpTimeline PlayFromStart)
      (:Update
        (Transformation|SetActorScale3D (Math|Vector|Lerp(Vector) (Variables|Default|GetactorCurrentScale) "0.500000, 0,1.500000" _squeeze))))
    (else
      (Timeline|JumpTimeline PlayFromStart))))

(event Custom|GetDamage
  (params (damageAmmount :type Integer))
  ;[1 1 1] Get damage +/-
  (if (> damageAmmount 0)
    (if (<= (+ (Variables|Default|GethealthCount) damageAmmount) (Variables|Default|GetmaxHealth))
      (Variables|Default|SethealthCount (+ (Variables|Default|GethealthCount) damageAmmount)))
    (elif (Variables|Default|GetcanGetDamage)
      (Variables|Default|SetcanGetDamage false)
      (Variables|Default|SethealthCount (+ (Variables|Default|GethealthCount) damageAmmount))
      (if (<= (Variables|Default|GethealthCount) 0)
        (CallFunction|Die)
        (else
          (bind _colortrack (Timeline|GetDamageTimeline PlayFromStart)
            (:Update
              (Sprite|SetSpriteColor (Variables|Default|GetSprite) _colortrack))
            (:Finished
              (Variables|Default|SetcanGetDamage true))))))))

(event Custom|StateCheck
  (bind _returnvalue (Transformation|GetVelocity))
  ;[1 1 1] State check
  (Variables|Default|SetisGoingUp (> (.z _returnvalue) 0.0))
  (Variables|Default|SetisGoingDown (< (.z _returnvalue) 0.0))
  (Variables|Default|SetisWalking (> (Math|Vector|VectorLength (Math|Vector|MakeVector (.x (Transformation|GetVelocity)) 0.0 0.0)) 0.0))
  (bind _newparam (CallFunction|SetAnimationState (Variables|Default|GetisDying) (Variables|Default|GetisAttacking) (Variables|Default|GetisGoingUp) (Variables|Default|GetisGoingDown) (Variables|Default|GetisCrouching) (Variables|Default|GetisWalking)))
  (Sprite|SetFlipbook (Variables|Default|GetSprite) _newparam))

(event EventOnLanded
  (params (Hit :type Hit%20Result%20Structure%20%28by%20ref%29))
  ;[1 1 1] Jumping
  (Variables|Default|SetjumpsCount 0)
  (Variables|Default|SetisCrouching true)
  (CallFunction|LandFX)
  (Utilities|FlowControl|Delay 0.15)
  (Variables|Default|SetisCrouching false))

(event EventTick
  (params (DeltaSeconds :type Float%20%28single-precision%29))
  (bind _capsulecomponent (Variables|Collision|GetCapsuleComponent))
  (bind _returnvalue (Transformation|GetWorldLocation _capsulecomponent))
  ;[1 1 1] Tick
  (CallFunction|StateCheck)
  (CallFunction|CheckSite)
  (if (not (Math|Vector|Equal(Vector) "0, 0, 0" (Math|Vector|MakeVector 0.0 (.y _returnvalue) 0.0) 0.0001))
    (Transformation|SetActorLocation (Math|Vector|MakeVector (.x _returnvalue) 0.0 (.z _returnvalue)) false false)))

(event Input|ActionEvents|InputActionJump
  (params (Key :type Key%20Structure))
  (bind _returnvalue (Transformation|GetVelocity))
  ;[1 1 1] Jumping
  (:Pressed
    (if (< (Variables|Default|GetjumpsCount) (Variables|Default|GetmaxJumps))
      (bind _result (Math|Integer|IncrementInt (Variables|Default|GetjumpsCount))
        (:%20%20
          (Variables|Default|SetjumpsCount _result)
          (if (> (.z _returnvalue) 0.0)
            (Character|LaunchCharacter (Math|Vector|MakeVector 0.0 0.0 (+ (* (.z (Transformation|GetVelocity)) -1.0) (* (Variables|Default|GetjumpBuffMultipler) 2.5e+02))) false false)
            (else
              (Character|LaunchCharacter (Math|Vector|MakeVector 0.0 0.0 (+ (Math|Float|Absolute(Float) (.z _returnvalue)) (* (Variables|Default|GetjumpBuffMultipler) 2.5e+02))) false false)))
          (CallFunction|JumpFX))))))

(event Input|ActionEvents|InputActionAttack
  (params (Key :type Key%20Structure))
  (bind _shootpoint (Variables|Default|GetShootPoint))
  ;[1 1 1] Attacking
  (:Pressed
    (if (Variables|Default|GetcanShoot)
      (Variables|Default|SetcanShoot false)
      (Variables|Default|SetisAttacking true)
      (Game|SpawnActorfromClass "/Game/BluePrints/Attacks/PlayerShoot1.PlayerShoot1_C" (Math|Transform|MakeTransform (Transformation|GetWorldLocation _shootpoint) (Transformation|GetWorldRotation _shootpoint) "0.500000,0.500000,0.500000") "AlwaysSpawn" 0 0)
      (Utilities|FlowControl|Delay 0.2)
      (Variables|Default|SetisAttacking false)
      (Utilities|FlowControl|Delay (- (Variables|Default|GetshootRate) 0.2))
      (Variables|Default|SetcanShoot true))))

(event Input|AxisEvents|InputAxisMoveRight
  (params (AxisValue :type Float%20%28single-precision%29))
  ;[1 1 1] Movement
  (Pawn|Input|AddMovementInput "1.000000, 0, 0" AxisValue false))

(fn ConstructionScript
  (Variables|Default|SetactorStartScale (Transformation|GetActorScale3D)))

(fn SetAnimationState
  (params (isDying :type Boolean) (isAttacking :type Boolean) (isGoingUp :type Boolean) (isGoingDown :type Boolean) (isCrouching :type Boolean) (isWalking :type Boolean))
  (if isDying
    (LocalVariables|SetStateFB "NewEnumerator9")
    (elif isAttacking
      (LocalVariables|SetStateFB "NewEnumerator7")
      (elif isGoingUp
        (LocalVariables|SetStateFB "NewEnumerator2")
        (elif isGoingDown
          (LocalVariables|SetStateFB "NewEnumerator6")
          (elif isCrouching
            (LocalVariables|SetStateFB "NewEnumerator5")
            (elif isWalking
              (LocalVariables|SetStateFB "NewEnumerator0")
              (else
                (LocalVariables|SetStateFB "NewEnumerator4"))))))))
  (return (Utilities|Select :Index (LocalVariables|GetStateFB) :NewEnumerator9 "/Game/Textures/Characters/Players/Player1/FlipBooks/FB_Player1_Death.FB_Player1_Death" :NewEnumerator7 "/Game/Textures/Characters/Players/Player1/FlipBooks/FB_Player1_Attack.FB_Player1_Attack" :NewEnumerator2 "/Game/Textures/Characters/Players/Player1/FlipBooks/FB_Player1_GoingUp.FB_Player1_GoingUp" :NewEnumerator6 "/Game/Textures/Characters/Players/Player1/FlipBooks/FB_Player1_GoingDown.FB_Player1_GoingDown" :NewEnumerator5 "/Game/Textures/Characters/Players/Player1/FlipBooks/FB_Player1_Crouch.FB_Player1_Crouch" :NewEnumerator0 "/Game/Textures/Characters/Players/Player1/FlipBooks/FB_Player1_Walkin.FB_Player1_Walkin" :NewEnumerator4 "/Game/Textures/Characters/Players/Player1/FlipBooks/FB_Player1_Idle.FB_Player1_Idle")))