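; PowerBall is an attack actor that kills enemies it hits and is spent on impact.
; Its Hit event runs a chain of casts against the range, aiming and side enemy base classes, destroying a matching actor outright with no damage step.
; The ball destroys itself on any hit, including non-enemies.
; The construction script sets it to half scale.
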(event Collision|EventHit
  (params (MyComp :type Primitive%20Component%20Object%20Reference) (Other :type Actor%20Object%20Reference) (OtherComp :type Primitive%20Component%20Object%20Reference) (bSelfMoved :type Boolean) (HitLocation :type Vector :default "0, 0, 0") (HitNormal :type Vector :default "0, 0, 0") (NormalImpulse :type Vector :default "0, 0, 0") (Hit :type Hit%20Result%20Structure%20%28by%20ref%29))
  (bind _asrange_enemy_base (Utilities|Casting|CastToRangeEnemyBase Other)
    (:then
      (Default|Destroy _asrange_enemy_base)
      (Actor|DestroyActor))
    (:CastFailed
      (bind _asaiming_enemy_base (Utilities|Casting|CastToAimingEnemyBase Other)
        (:then
          (Default|Destroy _asaiming_enemy_base)
          (Actor|DestroyActor))
        (:CastFailed
          (bind _asside_enemy_base (Utilities|Casting|CastToSideEnemyBase Other)
            (:then
              (Default|Destroy _asside_enemy_base)
              (Actor|DestroyActor))
            (:CastFailed
              (Actor|DestroyActor))))))))

(fn ConstructionScript
  (Transformation|SetActorScale3D "0.500000,0.500000,0.500000"))