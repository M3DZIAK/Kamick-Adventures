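; EnemyShoot2 is an enemy projectile with a flipbook sprite that damages Character1BP on contact.
; A Hit event damages the player and destroys the bullet on any collision, while box overlaps affect only the player and are ignored once IsDeath is set.
; A shared DestroyAnimation event, also triggered by a short lifetime timer, stops movement, plays the destroy flipbook and removes the actor after a brief delay.
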(event OnComponentBeginOverlap(Box)
  (params (OverlappedComponent :type Primitive%20Component%20Object%20Reference) (OtherActor :type Actor%20Object%20Reference) (OtherComp :type Primitive%20Component%20Object%20Reference) (OtherBodyIndex :type Integer) (bFromSweep :type Boolean) (SweepResult :type Hit%20Result%20Structure%20%28by%20ref%29))
  ;[1 1 1] Detection
  (bind _ascharacter_1bp (Utilities|Casting|CastToCharacter1BP OtherActor))
  (if (not (Variables|Default|GetisDeath))
    (Default|GetDamage _ascharacter_1bp -1)
    (CallFunction|DestroyAnimation)))

(event Custom|DestroyAnimation
  ;[1 1 1] Destroy
  (Variables|Default|SetisDeath true)
  (Components|Movement|StopMovementImmediately (Variables|Default|GetProjectileMovement))
  (Sprite|SetFlipbook (Variables|Default|GetPaperFlipbook) "/Game/Textures/Characters/Enemy4/FlipBooks/FB_E4Bullet_Destroy.FB_E4Bullet_Destroy")
  (Utilities|FlowControl|Delay 0.2)
  (Actor|DestroyActor))

(event Collision|EventHit
  (params (MyComp :type Primitive%20Component%20Object%20Reference) (Other :type Actor%20Object%20Reference) (OtherComp :type Primitive%20Component%20Object%20Reference) (bSelfMoved :type Boolean) (HitLocation :type Vector :default "0, 0, 0") (HitNormal :type Vector :default "0, 0, 0") (NormalImpulse :type Vector :default "0, 0, 0") (Hit :type Hit%20Result%20Structure%20%28by%20ref%29))
  ;[1 1 1] Detection
  (bind _ascharacter_1bp (Utilities|Casting|CastToCharacter1BP Other)
    (:then
      (Default|GetDamage _ascharacter_1bp -1)
      (CallFunction|DestroyAnimation))
    (:CastFailed
      (CallFunction|DestroyAnimation))))

(event EventBeginPlay
  ;[1 1 1] Start
  (Utilities|FlowControl|Delay 1.5)
  (CallFunction|DestroyAnimation))

(fn ConstructionScript)