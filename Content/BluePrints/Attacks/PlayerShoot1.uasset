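; PlayerShoot1 is the player's Paper2D bullet projectile, which destroys enemies on contact.
; On hit, a chain of casts destroys the range, aiming slime, side and fountain enemy types outright.
; Any hit, or a 1.5-second lifetime expiring, triggers a shared destroy event that halts the projectile movement, swaps to a burst flipbook, then removes the actor after a short delay.
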(event Custom|DestroyAnimation
  ;[1 1 1] Destroy
  (Components|Movement|StopMovementImmediately (Variables|Default|GetProjectileMovement))
  (Sprite|SetFlipbook (Variables|Default|GetPaperFlipbook) "/Game/Textures/Characters/Players/Player1/FlipBooks/FB_P1Bullet_Destroy.FB_P1Bullet_Destroy")
  (Utilities|FlowControl|Delay 0.2)
  (Actor|DestroyActor))

(event Collision|EventHit
  (params (MyComp :type Primitive%20Component%20Object%20Reference) (Other :type Actor%20Object%20Reference) (OtherComp :type Primitive%20Component%20Object%20Reference) (bSelfMoved :type Boolean) (HitLocation :type Vector :default "0, 0, 0") (HitNormal :type Vector :default "0, 0, 0") (NormalImpulse :type Vector :default "0, 0, 0") (Hit :type Hit%20Result%20Structure%20%28by%20ref%29))
  ;[1 1 1] Detection
  (bind _asrange_enemy_base (Utilities|Casting|CastToRangeEnemyBase Other)
    (:then
      (Default|Destroy _asrange_enemy_base)
      (CallFunction|DestroyAnimation))
    (:CastFailed
      (bind _asaiming_enemy_slime (Utilities|Casting|CastToAimingEnemySlime Other)
        (:then
          (Default|Destroy _asaiming_enemy_slime)
          (CallFunction|DestroyAnimation))
        (:CastFailed
          (bind _asside_enemy_base (Utilities|Casting|CastToSideEnemyBase Other)
            (:then
              (Default|Destroy _asside_enemy_base)
              (CallFunction|DestroyAnimation))
            (:CastFailed
              (bind _asfountain_enemy_1 (Utilities|Casting|CastToFountainEnemy1 Other)
                (:then
                  (Default|Destroy _asfountain_enemy_1)
                  (CallFunction|DestroyAnimation))
                (:CastFailed
                  (CallFunction|DestroyAnimation))))))))))

(event EventBeginPlay
  ;[1 1 1] Start
  (Utilities|FlowControl|Delay 1.5)
  (CallFunction|DestroyAnimation))

(fn ConstructionScript)