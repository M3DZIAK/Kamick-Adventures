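; Paper2D side-scroller player character with walking, multi-jump, projectile shooting and health, driven by input bindings or mobile events.
; Tick derives facing and flipbook state from velocity, with a brief crouch on landing.
; Jumps use LaunchCharacter with velocity compensation, while timelines add squash-and-stretch.
; Signed GetDamage heals or hurts with flashing invulnerability and death at zero health; mushroom pickups temporarily enlarge the character and boost jumps.
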(event Custom|BrownMushroomPickUp
  ;[1 1 1] BrownMushroomPickUp
  (bind _changescale (Timeline|PickUpTimeLine PlayFromStart)
    (:Update
      (Transformation|SetActorScale3D (Math|Vector|Lerp(Vector) (Variables|Default|GetactorStartScale) "2.000000,2.000000,2.000000" _changescale)))
    (:Finished
      (Transformation|SetActorScale3D "1.300000,1.300000,1.300000")
      (Variables|Default|SetjumpBuffMultipler (+ (Variables|Default|GetjumpBuffMultipler) 0.5))
      (Variables|Default|SetactorCurrentScale "1.300000,1.300000,1.300000")
      (Utilities|FlowControl|Delay 5.0)
      (Variables|Default|SetjumpBuffMultipler (- (Variables|Default|GetjumpBuffMultipler) 0.5))
      (Variables|Default|SetactorCurrentScale (Variables|Default|GetactorStartScale))
      (Transformation|SetActorScale3D (Variables|Default|GetactorCurrentScale)))))

(event Custom|moveCharacter%20mobile
  (params (speed :type Float%20%28single-precision%29))
  ;[1 1 1] Movement
  (Pawn|Input|AddMovementInput "1.000000, 0, 0" speed false))

(event Custom|CheckSite
  ;[1 1 1] Check site
  (Math|Float|CompareFloat (.X (Math|Vector|BreakVector (Transformation|GetVelocity))) 0.0
    (:>
      (Transformation|SetRelativeRotation (Variables|Default|GetSprite) "0, 0, 0" false false))
    (:<
      (Transformation|SetRelativeRotation (Variables|Default|GetSprite) "0.000000,180.000000,0.000000" false false))))

(event Custom|Die
  ;[1 1 1] Death
  (Pawn|Components|CharacterMovement|DisableMovement (Variables|Character|GetCharacterMovement))
  (Variables|Default|SetcanShoot false))

(event Custom|LandFX
  ;[1 1 1] LandFX
  (bind _squeeze (Timeline|LandTimeline PlayFromStart)
    (:Update
      (Transformation|SetActorScale3D (Math|Vector|Lerp(Vector) (Variables|Default|GetactorCurrentScale) "1.500000,0.000000,0.750000" _squeeze)))))

(event Custom|JumpMobile
  (bind _returnvalue (Transformation|GetVelocity))
  ;[1 1 1] Jumping
  (if (< (Variables|Default|GetjumpsCount) (Variables|Default|GetmaxJumps))
    (bind _result (Math|Integer|IncrementInt (Variables|Default|GetjumpsCount))
      (:%20%20
        (Variables|Default|SetjumpsCount _result)
        (if (> (.z _returnvalue) 0.0)
          (Character|LaunchCharacter (Math|Vector|MakeVector 0.0 0.0 (+ (* (.z (Transformation|GetVelocity)) -1.0) (* (Variables|Default|GetjumpBuffMultipler) 2.5e+02))) false false)
          (else
            (Character|LaunchCharacter (Math|Vector|MakeVector 0.0 0.0 (+ (Math|Float|Absolute(Float) (.z _returnvalue)) (* (Variables|Default|GetjumpBuffMultipler) 2.5e+02))) false false)))
        (CallFunction|JumpFX)))))

(event Custom|AttackMobile
  ;[1 1 1] Attacking
  (if (Variables|Default|GetcanShoot)
    (Variables|Default|SetcanShoot false)
    (Game|SpawnActorfromClass "/Game/BluePrints/Attacks/PowerBall.PowerBall_C" (Transformation|GetWorldTransform (Variables|Default|GetShootPoint)) "AlwaysSpawn" 0 0)
    (Utilities|FlowControl|Delay (Variables|Default|GetshootRate))
    (Variables|Default|SetcanShoot true)))

(event Custom|JumpFX
  ;[1 1 1] JumpFX
  (if (AI|Components|NavMovement|IsFalling (Variables|Character|GetCharacterMovement))
    (Effects|SpawnEmitteratLocation "/Game/Particles/DustParticle.DustParticle" (Transformation|GetWorldLocation (Variables|Default|GetBottomPoint)) "0, 0, 0" "0.300000,0.300000,0.300000")
    (bind _squeeze (Timeline|JumpTimeline PlayFromStart)
      (:Update
        (Transformation|SetActorScale3D (Math|Vector|Lerp(Vector) (Variables|Default|GetactorCurrentScale) "0.500000, 0,1.500000" _squeeze))))
    (else
      (Timeline|JumpTimeline PlayFromStart))))

(event Custom|GetDamage
  (params (damageAmmount :type Integer))
  ;[1 1 1] Get damage +/-
  (if (> damageAmmount 0)
    (if (<= (+ (Variables|Default|GethealthCount) damageAmmount) (Variables|Default|GetmaxHealth))
      (Variables|Default|SethealthCount (+ (Variables|Default|GethealthCount) damageAmmount)))
    (elif (Variables|Default|GetcanGetDamage)
      (Variables|Default|SetcanGetDamage false)
      (Variables|Default|SethealthCount (+ (Variables|Default|GethealthCount) damageAmmount))
      (if (<= (Variables|Default|GethealthCount) 0)
        (CallFunction|Die)
        (else
          (bind _colortrack (Timeline|GetDamageTimeline PlayFromStart)
            (:Update
              (Sprite|SetSpriteColor (Variables|Default|GetSprite) _colortrack))
            (:Finished
              (Variables|Default|SetcanGetDamage true))))))))

(event Custom|StateCheck
  ;[1 1 1] State check
  (if (!= (Math|Vector|VectorLength (Math|Vector|MakeVector 0.0 0.0 (.z (Transformation|GetVelocity)))) 0.0)
    (Variables|Default|SetisJumping true)
    (else
      (Variables|Default|SetisJumping false)))
  (Variables|Default|SetisWalking (> (Math|Vector|VectorLength (Math|Vector|MakeVector (.x (Transformation|GetVelocity)) 0.0 0.0)) 0.0))
  (bind _newparam (CallFunction|SetAnimationState (Variables|Default|GetisCrouching) (Variables|Default|GetisJumping) (Variables|Default|GetisWalking)))
  (Sprite|SetFlipbook (Variables|Default|GetSprite) _newparam))

(event EventOnLanded
  (params (Hit :type Hit%20Result%20Structure%20%28by%20ref%29))
  ;[1 1 1] Jumping
  (Variables|Default|SetjumpsCount 0)
  (Variables|Default|SetisCrouching true)
  (CallFunction|LandFX)
  (Utilities|FlowControl|Delay 0.15)
  (Variables|Default|SetisCrouching false))

(event EventTick
  (params (DeltaSeconds :type Float%20%28single-precision%29))
  ;[1 1 1] Tick
  (CallFunction|StateCheck)
  (CallFunction|CheckSite))

(event Input|ActionEvents|InputActionJump
  (params (Key :type Key%20Structure))
  (bind _returnvalue (Transformation|GetVelocity))
  ;[1 1 1] Jumping
  (:Pressed
    (if (< (Variables|Default|GetjumpsCount) (Variables|Default|GetmaxJumps))
      (bind _result (Math|Integer|IncrementInt (Variables|Default|GetjumpsCount))
        (:%20%20
          (Variables|Default|SetjumpsCount _result)
          (if (> (.z _returnvalue) 0.0)
            (Character|LaunchCharacter (Math|Vector|MakeVector 0.0 0.0 (+ (* (.z (Transformation|GetVelocity)) -1.0) (* (Variables|Default|GetjumpBuffMultipler) 2.5e+02))) false false)
            (else
              (Character|LaunchCharacter (Math|Vector|MakeVector 0.0 0.0 (+ (Math|Float|Absolute(Float) (.z _returnvalue)) (* (Variables|Default|GetjumpBuffMultipler) 2.5e+02))) false false)))
          (CallFunction|JumpFX))))))

(event Input|ActionEvents|InputActionAttack
  (params (Key :type Key%20Structure))
  ;[1 1 1] Attacking
  (:Pressed
    (if (Variables|Default|GetcanShoot)
      (Variables|Default|SetcanShoot false)
      (Game|SpawnActorfromClass "/Game/BluePrints/Attacks/PowerBall.PowerBall_C" (Transformation|GetWorldTransform (Variables|Default|GetShootPoint)) "AlwaysSpawn" 0 0)
      (Utilities|FlowControl|Delay (Variables|Default|GetshootRate))
      (Variables|Default|SetcanShoot true))))

(event Input|AxisEvents|InputAxisMoveRight
  (params (AxisValue :type Float%20%28single-precision%29))
  ;[1 1 1] Movement
  (Pawn|Input|AddMovementInput "1.000000, 0, 0" AxisValue false))

(fn ConstructionScript
  (Variables|Default|SetactorStartScale (Transformation|GetActorScale3D)))

(fn SetAnimationState
  (params (isCrouching :type Boolean) (isJumping :type Boolean) (isWalking :type Boolean))
  (if isCrouching
    (LocalVariables|SetStateFB "NewEnumerator5")
    (elif isJumping
      (LocalVariables|SetStateFB "NewEnumerator2")
      (elif isWalking
        (LocalVariables|SetStateFB "NewEnumerator0")
        (else
          (LocalVariables|SetStateFB "NewEnumerator4")))))
  (return (Utilities|Select :Index (LocalVariables|GetStateFB) :NewEnumerator0 "/Game/Textures/Characters/Flipbooks/Walking.Walking" :NewEnumerator2 "/Game/Textures/Characters/Flipbooks/Jumping.Jumping" :NewEnumerator4 "/Game/Textures/Characters/Flipbooks/Idle.Idle" :NewEnumerator5 "/Game/Textures/Characters/Flipbooks/Crouch.Crouch")))