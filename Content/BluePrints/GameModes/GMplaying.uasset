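; Gameplay game mode that tracks a level's timer, coins and pickups, and persists progress through SaveGameBP slots.
; Pickup handlers add coin value or forward mushroom effects to the player, while Tick counts time through a one-second Delay.
; Save events add money to the stored total, unlock the next map and record best times for three levels.
; Level 3 saves only its first record, as the improved-time save is disconnected.
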(event Custom|SaveRecord
  (bind _gametimeseconds (Variables|Default|GetgameTimeSeconds))
  (bind _gametimeminutes (Variables|Default|GetgameTimeMinutes))
  (bind _gametimeseconds_2 (Variables|Default|GetgameTimeSeconds))
  (bind _gametimeminutes_2 (Variables|Default|GetgameTimeMinutes))
  ;[1 1 1] Save record
  (bind _returnvalue (SaveGame|LoadGamefromSlot "maps"))
  (bind _assave_game_bp (Utilities|Casting|CastToSaveGameBP _returnvalue))
  (bind _output_get (Variables|Default|SetnowPlaying (Variables|/Game/BluePrints/Saving/SaveGameBP.SaveGameBP_C|GetnowMapPlaying _assave_game_bp)))
  (if (== _output_get 1)
    (bind _returnvalue_2 (SaveGame|DoesSaveGameExist "record1"))
    (if _returnvalue_2
      (bind _returnvalue_3 (SaveGame|LoadGamefromSlot "record1"))
      (bind _assave_game_bp_2 (Utilities|Casting|CastToSaveGameBP _returnvalue_3))
      (if (< (+ (* _gametimeminutes 100) _gametimeseconds) (+ (Variables|/Game/BluePrints/Saving/SaveGameBP.SaveGameBP_C|GetrecordLevel1sec _assave_game_bp_2) (* (Variables|/Game/BluePrints/Saving/SaveGameBP.SaveGameBP_C|GetrecordLevel1Min _assave_game_bp_2) 100)))
        (bind _returnvalue_4 (SaveGame|CreateSaveGameObject "/Game/BluePrints/Saving/SaveGameBP.SaveGameBP_C"))
        (Variables|/Game/BluePrints/Saving/SaveGameBP.SaveGameBP_C|SetrecordLevel1sec _returnvalue_4 _gametimeseconds)
        (Variables|/Game/BluePrints/Saving/SaveGameBP.SaveGameBP_C|SetrecordLevel1Min _returnvalue_4 _gametimeminutes)
        (SaveGame|SaveGametoSlot _returnvalue_4 "record1")
        (Variables|Default|SetnewRecord true :!label _label))
      (else
        (bind _returnvalue_5 (SaveGame|CreateSaveGameObject "/Game/BluePrints/Saving/SaveGameBP.SaveGameBP_C"))
        (Variables|/Game/BluePrints/Saving/SaveGameBP.SaveGameBP_C|SetrecordLevel1sec _returnvalue_5 (Variables|Default|GetgameTimeSeconds))
        (Variables|/Game/BluePrints/Saving/SaveGameBP.SaveGameBP_C|SetrecordLevel1Min _returnvalue_5 (Variables|Default|GetgameTimeMinutes))
        (SaveGame|SaveGametoSlot _returnvalue_5 "record1")
        (Variables|Default|SetnewRecord true :!label _label_2)))
    (elif (== _output_get 2)
      (bind _returnvalue_6 (SaveGame|DoesSaveGameExist "record2"))
      (if _returnvalue_6
        (bind _returnvalue_7 (SaveGame|LoadGamefromSlot "record2"))
        (bind _assave_game_bp_3 (Utilities|Casting|CastToSaveGameBP _returnvalue_7))
        (if (< (+ (* _gametimeminutes_2 100) _gametimeseconds_2) (+ (Variables|/Game/BluePrints/Saving/SaveGameBP.SaveGameBP_C|GetrecordLevel2sec _assave_game_bp_3) (* (Variables|/Game/BluePrints/Saving/SaveGameBP.SaveGameBP_C|GetrecordLevel2min _assave_game_bp_3) 100)))
          (bind _returnvalue_8 (SaveGame|CreateSaveGameObject "/Game/BluePrints/Saving/SaveGameBP.SaveGameBP_C"))
          (Variables|/Game/BluePrints/Saving/SaveGameBP.SaveGameBP_C|SetrecordLevel2sec _returnvalue_8 _gametimeseconds_2)
          (Variables|/Game/BluePrints/Saving/SaveGameBP.SaveGameBP_C|SetrecordLevel2min _returnvalue_8 _gametimeminutes_2)
          (SaveGame|SaveGametoSlot _returnvalue_8 "record2")
          (goto _label))
        (else
          (bind _returnvalue_9 (SaveGame|CreateSaveGameObject "/Game/BluePrints/Saving/SaveGameBP.SaveGameBP_C"))
          (Variables|/Game/BluePrints/Saving/SaveGameBP.SaveGameBP_C|SetrecordLevel2sec _returnvalue_9 (Variables|Default|GetgameTimeSeconds))
          (Variables|/Game/BluePrints/Saving/SaveGameBP.SaveGameBP_C|SetrecordLevel2min _returnvalue_9 (Variables|Default|GetgameTimeMinutes))
          (SaveGame|SaveGametoSlot _returnvalue_9 "record2")
          (goto _label_2)))
      (elif (== _output_get 3)
        (bind _returnvalue_10 (SaveGame|DoesSaveGameExist "record3"))
        (if _returnvalue_10
          (bind _returnvalue_11 (SaveGame|LoadGamefromSlot "record3"))
          (bind _assave_game_bp_4 (Utilities|Casting|CastToSaveGameBP _returnvalue_11))
          (if (< (+ (* (Variables|Default|GetgameTimeMinutes) 100) (Variables|Default|GetgameTimeSeconds)) (+ (Variables|/Game/BluePrints/Saving/SaveGameBP.SaveGameBP_C|GetrecordLevel3sec _assave_game_bp_4) (* (Variables|/Game/BluePrints/Saving/SaveGameBP.SaveGameBP_C|GetrecordLevel3min _assave_game_bp_4) 100)))
            (bind _returnvalue_12 (SaveGame|CreateSaveGameObject "/Game/BluePrints/Saving/SaveGameBP.SaveGameBP_C")))
          (else
            (bind _returnvalue_13 (SaveGame|CreateSaveGameObject "/Game/BluePrints/Saving/SaveGameBP.SaveGameBP_C"))
            (Variables|/Game/BluePrints/Saving/SaveGameBP.SaveGameBP_C|SetrecordLevel3sec _returnvalue_13 (Variables|Default|GetgameTimeSeconds))
            (Variables|/Game/BluePrints/Saving/SaveGameBP.SaveGameBP_C|SetrecordLevel3min _returnvalue_13 (Variables|Default|GetgameTimeMinutes))
            (SaveGame|SaveGametoSlot _returnvalue_13 "record3")
            (goto _label_2)))))))

(event Custom|SaveMoney
  ;[1 1 1] Save money
  (bind _returnvalue (SaveGame|DoesSaveGameExist "money"))
  (if _returnvalue
    (bind _returnvalue_2 (SaveGame|LoadGamefromSlot "money"))
    (bind _assave_game_bp (Utilities|Casting|CastToSaveGameBP _returnvalue_2))
    (bind _returnvalue_3 (SaveGame|CreateSaveGameObject "/Game/BluePrints/Saving/SaveGameBP.SaveGameBP_C"))
    (Variables|/Game/BluePrints/Saving/SaveGameBP.SaveGameBP_C|SetmoneyCount _returnvalue_3 (+ (Variables|/Game/BluePrints/Saving/SaveGameBP.SaveGameBP_C|GetmoneyCount _assave_game_bp) (Variables|Default|GetmoneyCount)))
    (SaveGame|SaveGametoSlot _returnvalue_3 "money")))

(event Custom|SaveMaps
  ;[1 1 1] SaveMaps
  (bind _returnvalue (SaveGame|DoesSaveGameExist "maps"))
  (if _returnvalue
    (bind _returnvalue_2 (SaveGame|LoadGamefromSlot "maps"))
    (bind _assave_game_bp (Utilities|Casting|CastToSaveGameBP _returnvalue_2))
    (SaveGame|CreateSaveGameObject "/Game/BluePrints/Saving/SaveGameBP.SaveGameBP_C")
    (if (== (Variables|/Game/BluePrints/Saving/SaveGameBP.SaveGameBP_C|GetlastMapUnlocked _assave_game_bp) (Variables|/Game/BluePrints/Saving/SaveGameBP.SaveGameBP_C|GetnowMapPlaying _assave_game_bp))
      (Variables|/Game/BluePrints/Saving/SaveGameBP.SaveGameBP_C|SetlastMapUnlocked _assave_game_bp (+ (Variables|/Game/BluePrints/Saving/SaveGameBP.SaveGameBP_C|GetlastMapUnlocked _assave_game_bp) 1))
      (SaveGame|SaveGametoSlot _assave_game_bp "maps"))))

(event EventBeginPlay
  ;[1 1 1] Start
  (bind _ascharacter_bp (Utilities|Casting|CastToCharacterBP (Game|Player|GetPlayerPawn 0)))
  (Variables|Default|SetplayerBP _ascharacter_bp)
  (bind _returnvalue (SaveGame|DoesSaveGameExist "characters"))
  (if _returnvalue
    (bind _returnvalue_2 (SaveGame|LoadGamefromSlot "characters"))
    (bind _assave_game_bp (Utilities|Casting|CastToSaveGameBP _returnvalue_2))
    (Variables|Default|SetcharacterID (Variables|/Game/BluePrints/Saving/SaveGameBP.SaveGameBP_C|GetcharacterId _assave_game_bp))))

(event EventTick
  (params (DeltaSeconds :type Float%20%28single-precision%29))
  ;[1 1 1] Update
  (if (Variables|Default|GetupdateTime)
    (Utilities|FlowControl|Delay 1.0)
    (bind _result (Math|Integer|IncrementInt (Variables|Default|GetgameTimeSeconds))
      (:%20%20
        (if (>= _result 60)
          (Math|Integer|IncrementInt (Variables|Default|GetgameTimeMinutes)
            (:%20%20
              (Variables|Default|SetgameTimeSeconds 0))))))))

(fn ConstructionScript)

(fn OnPickup
  (params (PickUpType :type Respawnable%20Base%20Object%20Reference))
  (Utilities|Casting|CastToPickUpBrownMushroom PickUpType)
  (Default|BrownMushroomPickUp (Variables|Default|GetplayerBP))
  (return))

(fn OnCollect
  (params (CollectableBase :type Not%20Respawnable%20Base%20Object%20Reference))
  (Utilities|Casting|CastToPickUpCoinBronze CollectableBase
    (:then
      (Variables|Default|SetmoneyCount (+ (Variables|Default|GetmoneyCount) 1))
      (return))
    (:CastFailed
      (Utilities|Casting|CastToPickUpCoinSilver CollectableBase
        (:then
          (Variables|Default|SetmoneyCount (+ (Variables|Default|GetmoneyCount) 2))
          (return))
        (:CastFailed
          (Utilities|Casting|CastToPickUpCoinGold CollectableBase
            (:then
              (Variables|Default|SetmoneyCount (+ (Variables|Default|GetmoneyCount) 3))
              (return))
            (:CastFailed
              (Utilities|Casting|CastToPickUpRedMushroom CollectableBase)
              (Default|GetDamage (Variables|Default|GetplayerBP) 1))))))))